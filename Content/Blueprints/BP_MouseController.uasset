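; BP_MouseController puts the TurnsSelector widget on screen for non-authority instances and connects its EndTurn button to ending the turn.
; As a workaround for unreliable viewport adding, Tick creates and adds a new widget on each of roughly the first thousand frames, stacking duplicates.
; Each copy's button release calls EndTurn, which is defined outside this graph.
; The OnClicked handler is empty and never bound.
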(event Custom|OnClicked_Event_0)

(event Custom|OnMouseRelease
  (Class|MouseController|EndTurn))

(event EventTick
  (params (DeltaSeconds :type Float%20%28single-precision%29))
  ;[1 1 1] Inconsistent Adding to Viewport lead to Misfunctionality. Try add 1,000 times. By then, functionality should work. Not sure why it didn't work, though. This is a disgusting fix.
  (Math|Integer|IncrementInt (Variables|Default|GetLimit)
    (:%20%20
      (if (< (Variables|Default|GetLimit) 1000)
        (Networking|SwitchHasAuthority
          (:Remote
            (bind _returnvalue (UserInterface|CreateWidget "/Game/UI/TurnsSelector.TurnsSelector_C"))
            (UserInterface|Viewport|AddtoViewport _returnvalue 0)
            (EventDispatchers|BindEventtoOnReleased (Variables|/Game/UI/TurnsSelector.TurnsSelector_C|GetEndTurn _returnvalue) (delegate Custom|OnMouseRelease))))))))

(fn ConstructionScript)